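; BP_Mouvement_Player is a 2D side-view player character that moves and jumps, using flipbook animation.
; BeginPlay adds the MC_Default Enhanced Input mapping context to the player controller.
; IA_Movement applies movement along the forward vector, flips the sprite by input sign and swaps walk/idle flipbooks; IA_Jump jumps, reusing those flipbooks.
; Older axis movement, controller-rotation and velocity-based animation logic remains disconnected.
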(event Custom|UpdateAnimation
  ;[1 1 1] Actual
  (Sprite|SetFlipbook (Variables|Default|GetSprite) (select (> (Math|Vector|VectorLength (Variables|/Script/Engine.MovementComponent|GetVelocity (Variables|Character|GetCharacterMovement))) 0.0) "/Game/Asset/Assets_Marine/Animtion_Nuage_Blanc_Walk.Animtion_Nuage_Blanc_Walk" "/Game/Asset/Assets_Marine/Animtion_Nuage_Blanc_Idle.Animtion_Nuage_Blanc_Idle")))

(event Custom|UpdateControlAnimation
  ;[1 1 1] Old methods
)

(event Input|EnhancedActionEvents|EnhancedInputActionIA_Movement
  (params (ActionValue :type Float%20%28double-precision%29) (ElapsedSeconds :type Float%20%28double-precision%29) (TriggeredSeconds :type Float%20%28double-precision%29) (InputAction :type Input%20Action%20Object%20Reference :default "/Game/BluePrint/IA_Movement.IA_Movement"))
  ;[1 1 1] Test/Proposition
  (:Triggered
    (Pawn|Input|AddMovementInput (Transformation|GetActorForwardVector) ActionValue false)
    (Sprite|SetFlipbook (Variables|Default|GetSprite) "/Game/Asset/Assets_Marine/Animtion_Nuage_Blanc_Walk.Animtion_Nuage_Blanc_Walk")
    (if (> ActionValue 0.0)
      (Transformation|SetWorldRotation (Variables|Default|GetSprite) "0, 0, 0" false false)
      (else
        (Transformation|SetWorldRotation (Variables|Default|GetSprite) "0.000000,-180.000000,0.000000" false false))))
  (:Completed
    (Sprite|SetFlipbook (Variables|Default|GetSprite) "/Game/Asset/Assets_Marine/Animtion_Nuage_Blanc_Idle.Animtion_Nuage_Blanc_Idle")))

(event Input|EnhancedActionEvents|EnhancedInputActionIA_Jump
  (params (ActionValue :type Boolean) (ElapsedSeconds :type Float%20%28double-precision%29) (TriggeredSeconds :type Float%20%28double-precision%29) (InputAction :type Input%20Action%20Object%20Reference :default "/Game/BluePrint/IA_Jump.IA_Jump"))
  (bind _sprite (Variables|Default|GetSprite))
  ;[1 1 1] Test/Proposition
  (:Triggered
    (Character|Jump)
    (Components|Timeline|SetLooping _sprite false)
    (Sprite|SetFlipbook _sprite "/Game/Asset/Assets_Marine/Animtion_Nuage_Blanc_Walk.Animtion_Nuage_Blanc_Walk")
    (if (== (.Z (Math|Vector|BreakVector (Transformation|GetVelocity))) 0.0)
      (Components|Timeline|SetLooping _sprite true)
      (Audio|Components|Audio|Play _sprite)
      (Sprite|SetFlipbook _sprite "/Game/Asset/Assets_Marine/Animtion_Nuage_Blanc_Idle.Animtion_Nuage_Blanc_Idle"))))

(event EventTick
  (params (DeltaSeconds :type Float%20%28single-precision%29))
  ;[1 1 1] Actual
)

(event EventBeginPlay
  ;[1 1 1] Test/Proposition
  (bind _asbp_player_controller (Utilities|Casting|CastToBP_PlayerController (Pawn|GetController)))
  (Input|AddMappingContext (PlayerController|LocalPlayerSubsystems|GetEnhancedInputLocalPlayerSubsystem _asbp_player_controller) "/Game/BluePrint/MC_Default.MC_Default" 0 "(bIgnoreAllPressedKeysUntilRelease=True,bForceImmediately=False)"))

(event Input|AxisEvents|InputAxisMoveRight
  (params (AxisValue :type Float%20%28single-precision%29))
  ;[1 1 1] Old methods
)

(fn ConstructionScript)